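; Overworld day-night actor that swaps cloud and pillar Niagara effects (Awan/Api, cloud/fire) as the sun turns.
; BeginPlay hides the two Tiang (pillar) effects, then Tick checks whether the DirectionalLight pitch is at least zero.
; Two DoOnce gates reset each other, so ToggleAwanApi runs once per sign change, flipping the Cloud flag and both pairs' visibility.
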(event `self.ReceiveBeginPlay`
  (`parent.ReceiveBeginPlay`)
  (`SceneComponent.SetVisibility` (`NiagaraActor.NiagaraComponent` (`self.tiang1`)) false false)
  (`SceneComponent.SetVisibility` (`NiagaraActor.NiagaraComponent` (`self.tiang2`)) false false))

(event `self.ReceiveTick`
  (params (DeltaSeconds :type "Float (single-precision)"))
  (bind (_returnvalue_roll _returnvalue_pitch) (`KismetMathLibrary.BreakRotator` (`SceneComponent.K2_GetComponentRotation` (`self.DirectionalLight`))))
  (`parent.ReceiveTick` DeltaSeconds)
  (`|ExecutionSequence`
    (:`then_0`
      (if (>= _returnvalue_pitch 0.0)
        (`/Engine/EditorBlueprintResources/StandardMacros.DoOnce` false :!label _label
          (:`Completed`
            (`self.ToggleAwanApi`)
            (goto _label_2 :!via `Reset`)))
        (else
          (`/Engine/EditorBlueprintResources/StandardMacros.DoOnce` false :!label _label_2
            (:`Completed`
              (`self.ToggleAwanApi`)
              (goto _label :!via `Reset`))))))))

(fn `ToggleAwanApi`
  (if (`self.cloud`)
    (set `self.cloud` false)
    (`SceneComponent.SetVisibility` (`NiagaraActor.NiagaraComponent` (`self.tiang1`)) true false)
    (`SceneComponent.SetVisibility` (`NiagaraActor.NiagaraComponent` (`self.tiang2`)) true false)
    (`SceneComponent.SetVisibility` (`NiagaraActor.NiagaraComponent` (`self.cloud 1`)) false false)
    (`SceneComponent.SetVisibility` (`NiagaraActor.NiagaraComponent` (`self.cloud 2`)) false false)
    (else
      (set `self.cloud` true)
      (`SceneComponent.SetVisibility` (`NiagaraActor.NiagaraComponent` (`self.tiang1`)) false false)
      (`SceneComponent.SetVisibility` (`NiagaraActor.NiagaraComponent` (`self.tiang2`)) false false)
      (`SceneComponent.SetVisibility` (`NiagaraActor.NiagaraComponent` (`self.cloud 1`)) true false)
      (`SceneComponent.SetVisibility` (`NiagaraActor.NiagaraComponent` (`self.cloud 2`)) true false))))

(fn `UserConstructionScript`
  (`parent.UserConstructionScript`))