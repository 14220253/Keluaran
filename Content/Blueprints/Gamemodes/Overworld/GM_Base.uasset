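; Base game mode for the overworld that holds game stage progress, hint data, the world widget and an indicator target.
; GameStageIndex selects the current hint's video, audio and padded duration from GameStages, and ToNextGamestage increments it.
; It creates the WBP_World widget on request; SetHint always passes it the first entry of a separate Hints array.
; BeginPlay is empty, so all behavior runs through functions called from elsewhere.
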(event `self.ReceiveBeginPlay`)

(fn `CreateOverworldWidget`
  (bind _returnvalue (`|CreateWidget` "/Game/Blueprints/UI/WBP_World.WBP_World_C"))
  (bind _output_get (set `self.WorldWidget` _returnvalue))
  (`UserWidget.AddToViewport` _output_get -1))

(fn `GetCurrentHint`
  (returns (SourceVideo :type "FileMediaSource Object Reference") (Audio :type "SoundWave Object Reference") (Duration :type "Float (double-precision)"))
  (bind _gamestages_hints (break `/Game/Blueprints/Gamemodes/Overworld/S_GameStage` (`self.GameStages`)))
  (bind (_output_sourcevideo _output_audio _output_videoduration) (break `/Game/Blueprints/Gamemodes/Overworld/S_Hint` (`|GetArrayItem` _gamestages_hints (`self.GameStageIndex`))))
  (return _output_sourcevideo _output_audio (+ _output_videoduration 1.0)))

(fn `SetHint`
  (`/Game/Blueprints/UI/WBP_World.SetHint` (`self.WorldWidget`) (`|GetArrayItem` (`self.Hints`))))

(fn `SetIndicatorTarget`
  (params (Object :type "/Game/Blueprints/random/BP_Trigger Object Reference"))
  (set `self.IndicatorTarget` Object))

(fn `ToNextGamestage`
  (`/Engine/EditorBlueprintResources/StandardMacros.IncrementInt` (`self.GameStageIndex`)))

(fn `UserConstructionScript`)