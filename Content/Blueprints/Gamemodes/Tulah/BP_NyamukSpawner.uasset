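; Spawner actor for the Tulah game mode that periodically creates BP_Nyamuktes actors (nyamuk, mosquito) during Stage 1.
; Tick polls the GMBP_Tulah stage, activates the root component, and uses a DoOnce reset by a Delay to repeat the spawn every 30 seconds.
; Spawn places each actor slightly above the root's location, ignoring collisions.
; The node that would deactivate the root is unconnected and never runs.
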(event `self.ReceiveBeginPlay`)

(event `self.ReceiveTick`
  (params (DeltaSeconds :type "Float (single-precision)"))
  (bind _asgmbp_tulah (cast `/Game/Blueprints/Gamemodes/Tulah/GMBP_Tulah` (`GameplayStatics.GetGameMode`)))
  (if (== (`/Game/Blueprints/Gamemodes/Tulah/GMBP_Tulah.Stage` _asgmbp_tulah) 1)
    (`ActorComponent.SetActive` (`self.DefaultSceneRoot`) true false)
    (`/Engine/EditorBlueprintResources/StandardMacros.DoOnce` false :!label _label
      (:`Completed`
        (`self.Spawn`)
        (`KismetSystemLibrary.Delay` 30.0)
        (goto _label :!via `Reset`)))))

(fn `Spawn`
  (`|SpawnActorFromClass` "/Game/Blueprints/Gamemodes/Tulah/BP_Nyamuktes.BP_Nyamuktes_C" (`KismetMathLibrary.MakeTransform` (+ (`SceneComponent.K2_GetComponentLocation` (`self.DefaultSceneRoot`)) (0.0 0.0 10.0)) (`KismetMathLibrary.MakeRotator` 0.0)) "AlwaysSpawn" "MultiplyWithRoot" null null))

(fn `UserConstructionScript`)