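; BP_Nyamuktes is a chasing enemy pawn for the Tulah game mode that drains score on contact.
; Tick reissues AIMoveTo toward player 0's location every frame.
; Capsule overlaps with any other capsule component toggle PlayerColliding, without checking that it belongs to the player.
; While set, Tick subtracts points from GMBP_Tulah's Score, throttled by a DoOnce that resets after a short delay.
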(event `self.ReceiveTick`
  (params (DeltaSeconds :type "Float (single-precision)"))
  (`|ExecutionSequence`
    (:`then_0`
      (`|AIMoveTo` self (`self.K2_GetActorLocation` (`GameplayStatics.GetPlayerPawn` 0)) null 50.0 true))
    (:`then_1`
      (if (`self.PlayerColliding`)
        (`/Engine/EditorBlueprintResources/StandardMacros.DoOnce` false :!label _label
          (:`Completed`
            (bind _asgmbp_tulah (cast `/Game/Blueprints/Gamemodes/Tulah/GMBP_Tulah` (`GameplayStatics.GetGameMode`)))
            (set `/Game/Blueprints/Gamemodes/Tulah/GMBP_Tulah.Score` (- (`/Game/Blueprints/Gamemodes/Tulah/GMBP_Tulah.Score` _asgmbp_tulah) 10) _asgmbp_tulah)
            (`KismetSystemLibrary.Delay` 0.5)
            (goto _label :!via `Reset`)))))))

(event `self.CapsuleComponent.OnComponentBeginOverlap`
  (params (OverlappedComponent :type "PrimitiveComponent Object Reference") (OtherActor :type "Actor Object Reference") (OtherComp :type "PrimitiveComponent Object Reference") (OtherBodyIndex :type Integer) (bFromSweep :type Boolean) (SweepResult :type "HitResult Structure (by ref)"))
  (cast `CapsuleComponent` OtherComp)
  (set `self.PlayerColliding` true))

(event `self.CapsuleComponent.OnComponentEndOverlap`
  (params (OverlappedComponent :type "PrimitiveComponent Object Reference") (OtherActor :type "Actor Object Reference") (OtherComp :type "PrimitiveComponent Object Reference") (OtherBodyIndex :type Integer))
  (cast `CapsuleComponent` OtherComp)
  (set `self.PlayerColliding` false))

(fn `DrawDebugCapsule`
  (params (capsule :type "CapsuleComponent Object Reference"))
  (`KismetSystemLibrary.DrawDebugCapsule` (`SceneComponent.K2_GetComponentLocation` capsule) (`CapsuleComponent.GetScaledCapsuleHalfHeight` capsule) (`CapsuleComponent.GetScaledCapsuleRadius` capsule) (`SceneComponent.K2_GetComponentRotation` capsule) (struct :`R` 1.0 :`G` 0.895311 :`A` 1.0) 1.0 1.0))

(fn `UserConstructionScript`)