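; Spawner actor that periodically spawns BP_Kodok (frog) actors during stage 0 of the Tulah game mode.
; Tick checks the game mode stage and runs a reset-after-delay DoOnce loop that rolls a roughly even chance to spawn at random intervals.
; Each frog appears slightly above the spawner, with yaw toward the player snapped to 90-degree steps.
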(event `self.ReceiveBeginPlay`)

(event `self.ReceiveTick`
  (params (DeltaSeconds :type "Float (single-precision)"))
  (bind _defaultsceneroot (`self.DefaultSceneRoot`))
  (bind _asgmbp_tulah (cast `/Game/Blueprints/Gamemodes/Tulah/GMBP_Tulah` (`GameplayStatics.GetGameMode`)))
  (if (== (`/Game/Blueprints/Gamemodes/Tulah/GMBP_Tulah.Stage` _asgmbp_tulah) 0)
    (`ActorComponent.SetActive` _defaultsceneroot true false)
    (`/Engine/EditorBlueprintResources/StandardMacros.DoOnce` false :!label _label
      (:`Completed`
        (if (<= (`KismetMathLibrary.RandomIntegerInRange` 0 100) 50)
          (`self.Spawn`))
        (`KismetSystemLibrary.Delay` (`KismetMathLibrary.RandomFloatInRange` 5.0 10.0))
        (goto _label :!via `Reset`)))
    (else
      (`ActorComponent.SetActive` _defaultsceneroot false false))))

(fn `Spawn`
  (bind _returnvalue (`SceneComponent.K2_GetComponentLocation` (`self.DefaultSceneRoot`)))
  (bind (_returnvalue_roll _returnvalue_pitch _returnvalue_yaw) (`KismetMathLibrary.BreakRotator` (`KismetMathLibrary.FindLookAtRotation` _returnvalue (`self.K2_GetActorLocation` (`GameplayStatics.GetPlayerPawn` 0)))))
  (`|SpawnActorFromClass` "/Game/Blueprints/Gamemodes/Tulah/BP_Kodok.BP_Kodok_C" (`KismetMathLibrary.MakeTransform` (+ _returnvalue (0.0 0.0 10.0)) (`KismetMathLibrary.MakeRotator` 0.0 0.0 (`KismetMathLibrary.Conv_IntToDouble` (* (`KismetMathLibrary.Round` (/ _returnvalue_yaw 90.0)) 90)))) "AlwaysSpawn" "MultiplyWithRoot" null null))

(fn `UserConstructionScript`)