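; Spawner for BP_HujanEs (hail) during Stage 3 of the Tulah game mode.
; Tick moves its root to the player while that stage runs and deactivates it otherwise.
; A Delay on Tick paces spawns to about one per second, at random navigable points near the player.
; A counter makes every eleventh spawn appear directly above the player instead.
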(event `self.ReceiveBeginPlay`)

(event `self.ReceiveTick`
  (params (DeltaSeconds :type "Float (single-precision)"))
  (bind _returnvalue (`self.K2_GetActorLocation` (`GameplayStatics.GetPlayerPawn` 0)))
  (bind _asgmbp_tulah (cast `/Game/Blueprints/Gamemodes/Tulah/GMBP_Tulah` (`GameplayStatics.GetGameMode`)))
  (if (== (`/Game/Blueprints/Gamemodes/Tulah/GMBP_Tulah.Stage` _asgmbp_tulah) 3)
    (`ActorComponent.SetActive` (`self.DefaultSceneRoot`) true false)
    (`|ExecutionSequence`
      (:`then_0`
        (`SceneComponent.K2_SetWorldLocation` (`self.DefaultSceneRoot`) _returnvalue false false))
      (:`then_1`
        (`KismetSystemLibrary.Delay` 1.0)
        (if (== (`self.Counter`) 10)
          (`|SpawnActorFromClass` "/Game/Blueprints/Gamemodes/Tulah/BP_HujanEs.BP_HujanEs_C" (`KismetMathLibrary.MakeTransform` (+ _returnvalue (0.0 0.0 100.0))) "Undefined" "MultiplyWithRoot" null null)
          (set `self.Counter` 0)
          (else
            (bind _randomlocation (`NavigationSystemV1.K2_GetRandomLocationInNavigableRadius` _returnvalue 500.0 null null))
            (`|SpawnActorFromClass` "/Game/Blueprints/Gamemodes/Tulah/BP_HujanEs.BP_HujanEs_C" (`KismetMathLibrary.MakeTransform` (+ _randomlocation (0.0 0.0 25.0))) "Undefined" "MultiplyWithRoot" null null)
            (`/Engine/EditorBlueprintResources/StandardMacros.IncrementInt` (`self.Counter`))))))
    (else
      (`ActorComponent.SetActive` (`self.DefaultSceneRoot`) false false))))

(fn `UserConstructionScript`)