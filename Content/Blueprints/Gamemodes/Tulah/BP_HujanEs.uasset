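; BP_HujanEs is a hail ("hujan es") hazard actor for the Tulah game mode that costs points on contact.
; On BeginPlay it activates its Niagara effect and destroys itself three seconds later.
; Tick moves only the collision Sphere downward at constant speed, without acceleration.
; Any capsule component overlapping the Sphere deducts score through GMBP_Tulah, and the actor persists after the hit.
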(event `self.ReceiveBeginPlay`
  (`ActorComponent.Activate` (`self.Niagara`) false)
  (`KismetSystemLibrary.Delay` 3.0)
  (`self.K2_DestroyActor`))

(event `self.ReceiveTick`
  (params (DeltaSeconds :type "Float (single-precision)"))
  (`SceneComponent.K2_AddWorldOffset` (`self.Sphere`) (`KismetMathLibrary.MakeVector` 0.0 0.0 (* -9.8 DeltaSeconds)) false false))

(event `self.Sphere.OnComponentBeginOverlap`
  (params (OverlappedComponent :type "PrimitiveComponent Object Reference") (OtherActor :type "Actor Object Reference") (OtherComp :type "PrimitiveComponent Object Reference") (OtherBodyIndex :type Integer) (bFromSweep :type Boolean) (SweepResult :type "HitResult Structure (by ref)"))
  (cast `CapsuleComponent` OtherComp)
  (bind _asgmbp_tulah (cast `/Game/Blueprints/Gamemodes/Tulah/GMBP_Tulah` (`GameplayStatics.GetGameMode`)))
  (`/Game/Blueprints/Gamemodes/Tulah/GMBP_Tulah.AddScore` _asgmbp_tulah -10))

(fn `UserConstructionScript`)