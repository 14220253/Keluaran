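; BP_Trigger_LV9 is a trigger actor, apparently for level 9, that advances the slideshow and teleports the player.
; When the third-person character overlaps its collision, it starts the next slide on GM_Base's SlideshowWidget and passes it the quiz, close behavior and next-level settings.
; It then calls CreateNextTrigger on the widget with itself and moves player pawn 0 to a hardcoded location.
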(event `self.collision.OnComponentBeginOverlap`
  (params (OverlappedComponent :type "PrimitiveComponent Object Reference") (OtherActor :type "Actor Object Reference") (OtherComp :type "PrimitiveComponent Object Reference") (OtherBodyIndex :type Integer) (bFromSweep :type Boolean) (SweepResult :type "HitResult Structure (by ref)"))
  (cast `/Game/ThirdPerson/Blueprints/BP_ThirdPersonCharacter` OtherActor)
  (bind _asgm_base (cast `/Game/Blueprints/Gamemodes/Overworld/GM_Base` (`GameplayStatics.GetGameMode`)))
  (bind _slideshowwidget (`/Game/Blueprints/Gamemodes/Overworld/GM_Base.SlideshowWidget` _asgm_base))
  (`/Game/Blueprints/Gamemodes/Slideshow/WBP_SlideShow.StartNextSlide` _slideshowwidget)
  (set `/Game/Blueprints/Gamemodes/Slideshow/WBP_SlideShow.GoQuizThenNextLevel` (`self.GoQuizThenNextLevel`) _slideshowwidget)
  (set `/Game/Blueprints/Gamemodes/Slideshow/WBP_SlideShow.GoNextLevelAfterClose` (`self.Go Next Level After Close`) _slideshowwidget)
  (set `/Game/Blueprints/Gamemodes/Slideshow/WBP_SlideShow.NextLevel` (`self.Next Level`) _slideshowwidget)
  (`/Game/Blueprints/Gamemodes/Slideshow/WBP_SlideShow.CreateNextTrigger` _slideshowwidget self)
  (`self.K2_SetActorLocation` (`GameplayStatics.GetPlayerPawn` 0) (-41810.0 3410.0 26430.0) false true))

(fn `UserConstructionScript`
  (`parent.UserConstructionScript`))