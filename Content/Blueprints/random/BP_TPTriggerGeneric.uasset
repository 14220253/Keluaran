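; Trigger box that teleports BP_ThirdPersonCharacter to the first "TPTarget" static mesh actor, then plays a parting-sea effect.
; A Timeline pushes "LautKiri" and "LautKanan" tagged actors in opposite directions along world Y, then destroys "LautBorder" actors when finished.
; Offsets accumulate on each Timeline update, so travel distance depends on frame rate.
; All targets are found by actor tag at runtime.
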(event `self.Box.OnComponentBeginOverlap`
  (params (OverlappedComponent :type "PrimitiveComponent Object Reference") (OtherActor :type "Actor Object Reference") (OtherComp :type "PrimitiveComponent Object Reference") (OtherBodyIndex :type Integer) (bFromSweep :type Boolean) (SweepResult :type "HitResult Structure (by ref)"))
  (bind _asbp_third_person_character (cast `/Game/ThirdPerson/Blueprints/BP_ThirdPersonCharacter` OtherActor))
  (bind _outactors (`GameplayStatics.GetAllActorsWithTag` "TPTarget"))
  (bind _asstatic_mesh_actor (cast `StaticMeshActor` (`|GetArrayItem` _outactors)))
  (`SceneComponent.K2_SetWorldLocation` (`Character.CapsuleComponent` _asbp_third_person_character) (`SceneComponent.K2_GetComponentLocation` (`StaticMeshActor.StaticMeshComponent` _asstatic_mesh_actor)) false true)
  (bind (_direction _offset) (`Timeline|Timeline` :!via `PlayFromStart`)
    (:`Update`
      (`|ExecutionSequence`
        (:`then_0`
          (bind _outactors_2 (`GameplayStatics.GetAllActorsWithTag` "LautKiri"))
          (bind _outactors_3 (`GameplayStatics.GetAllActorsWithTag` "LautKanan")))
        (:`then_1`
          (for _array_element _outactors_2
            (bind _returnvalue (* _offset 20.0))
            (`self.K2_AddActorWorldOffset` _array_element (`KismetMathLibrary.MakeVector` 0.0 _returnvalue) false false)))
        (:`then_2`
          (for _array_element_2 _outactors_3
            (`self.K2_AddActorWorldOffset` _array_element_2 (`KismetMathLibrary.MakeVector` 0.0 (* _returnvalue -1.0)) false false)))))
    (:`Finished`
      (bind _outactors_4 (`GameplayStatics.GetAllActorsWithTag` "LautBorder"))
      (for _array_element_3 _outactors_4
        (`self.K2_DestroyActor` _array_element_3)))))

(fn `UserConstructionScript`)