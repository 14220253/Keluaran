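; BP_TPTriggerLaut is a trigger that teleports the player to a linked point and moves the sea ("Laut") actors apart or together.
; On box overlap, it casts to BP_ThirdPersonCharacter and teleports the capsule to the Connection's PointSet, if Connection is set.
; A timeline then applies incremental world Y offsets each update, in opposite directions for actors tagged LautKiri (left) and LautKanan (right).
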(event `self.Box.OnComponentBeginOverlap`
  (params (OverlappedComponent :type "PrimitiveComponent Object Reference") (OtherActor :type "Actor Object Reference") (OtherComp :type "PrimitiveComponent Object Reference") (OtherBodyIndex :type Integer) (bFromSweep :type Boolean) (SweepResult :type "HitResult Structure (by ref)"))
  (if (!= (`self.connection`) null)
    (bind _asbp_third_person_character (cast `/Game/ThirdPerson/Blueprints/BP_ThirdPersonCharacter` OtherActor))
    (`SceneComponent.K2_SetWorldLocation` (`Character.CapsuleComponent` _asbp_third_person_character) (`SceneComponent.K2_GetComponentLocation` (`/Game/Blueprints/random/BP_TPTriggerLaut.PointSet` (`self.connection`))) false true)
    (bind (_direction _offset) (`Timeline|Timeline` :!via `PlayFromStart`)
      (:`Update`
        (`|ExecutionSequence`
          (:`then_0`
            (bind _outactors (`GameplayStatics.GetAllActorsWithTag` "LautKiri"))
            (bind _outactors_2 (`GameplayStatics.GetAllActorsWithTag` "LautKanan")))
          (:`then_1`
            (for _array_element _outactors
              (bind _returnvalue (* _offset 20.0))
              (`self.K2_AddActorWorldOffset` _array_element (`KismetMathLibrary.MakeVector` 0.0 _returnvalue) false false)))
          (:`then_2`
            (for _array_element_2 _outactors_2
              (`self.K2_AddActorWorldOffset` _array_element_2 (`KismetMathLibrary.MakeVector` 0.0 (* _returnvalue -1.0)) false false))))))))

(fn `UserConstructionScript`)