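; BP_NPC is an interactable non-player character that becomes the player's current dialog target when the player is nearby.
; Box overlap sets or clears CurrentNPC on the third-person character and toggles an outline by swapping the mesh overlay material.
; When touch controls are in use, it also enables or disables the dialog button on the UI_TouchSimple widget.
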(event `self.Box.OnComponentBeginOverlap`
  (params (OverlappedComponent :type "PrimitiveComponent Object Reference") (OtherActor :type "Actor Object Reference") (OtherComp :type "PrimitiveComponent Object Reference") (OtherBodyIndex :type Integer) (bFromSweep :type Boolean) (SweepResult :type "HitResult Structure (by ref)"))
  (bind _asbp_third_person_character (cast `/Game/ThirdPerson/Blueprints/BP_ThirdPersonCharacter` OtherActor))
  (`/Game/ThirdPerson/Blueprints/BP_ThirdPersonCharacter.SetCurrentNPC` _asbp_third_person_character self)
  (`self.EnableOutline`)
  (bind _asbp_third_person_player_controller (cast `/Game/ThirdPerson/Blueprints/BP_ThirdPersonPlayerController` (`GameplayStatics.GetPlayerController` 0)))
  (if (`/Game/ThirdPerson/Blueprints/BP_ThirdPersonPlayerController.Should Use Touch Controls` _asbp_third_person_player_controller)
    (bind _foundwidgets (`WidgetBlueprintLibrary.GetAllWidgetsOfClass` "/Game/Input/Touch/UI_TouchSimple.UI_TouchSimple_C"))
    (`/Game/Input/Touch/UI_TouchSimple.EnableDialogButton` (`|GetArrayItem` _foundwidgets))))

(event `self.Box.OnComponentEndOverlap`
  (params (OverlappedComponent :type "PrimitiveComponent Object Reference") (OtherActor :type "Actor Object Reference") (OtherComp :type "PrimitiveComponent Object Reference") (OtherBodyIndex :type Integer))
  (bind _asbp_third_person_character (cast `/Game/ThirdPerson/Blueprints/BP_ThirdPersonCharacter` OtherActor))
  (set `/Game/ThirdPerson/Blueprints/BP_ThirdPersonCharacter.CurrentNPC` null _asbp_third_person_character)
  (`self.DisableOutline`)
  (if (`/Game/ThirdPerson/Blueprints/BP_ThirdPersonPlayerController.Should Use Touch Controls` (stale `self.Box.OnComponentBeginOverlap` _asbp_third_person_player_controller))
    (bind _foundwidgets (`WidgetBlueprintLibrary.GetAllWidgetsOfClass` "/Game/Input/Touch/UI_TouchSimple.UI_TouchSimple_C"))
    (`/Game/Input/Touch/UI_TouchSimple.DisableDialogButton` (`|GetArrayItem` _foundwidgets))))

(fn `DisableOutline`
  (`MeshComponent.SetOverlayMaterial` (`self.Mesh`) "/Game/Material/M_None.M_None"))

(fn `EnableOutline`
  (`MeshComponent.SetOverlayMaterial` (`self.Mesh`) "/Game/Material/M_NPCOutline.M_NPCOutline"))

(fn `UserConstructionScript`)